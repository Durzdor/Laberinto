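; Player Blueprint providing walking, strafing and sprinting, with a light that flickers through a timeline started at BeginPlay.
; Input actions set direction flags that Tick turns into swept local offsets, without delta-time scaling.
; Sprint raises forward speed and swaps the sideways offset to Strafe, while backward movement always uses Walk.
; Rotation and clock logic is present but never runs.
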(event `self.ReceiveTick`
  (params (DeltaSeconds :type "Float (single-precision)"))
  (`|ExecutionSequence`
    (:`then_0`
      ;[1 1 1] MoveForward
      (if (`self.AllowForward`)
        (`self.K2_AddActorLocalOffset` (`self.Speed`) true)))
    (:`then_1`
      ;[1 1 1] MoveBackward
      (if (`self.AllowBackward`)
        (`self.K2_AddActorLocalOffset` (* (`self.Walk`) -1) true)))
    (:`then_2`
      ;[1 1 1] MoveLeft
      (if (and (`self.AllowLeft`) (`self.Sprinting`))
        (`self.K2_AddActorLocalOffset` (`self.Strafe`) true)
        (elif (`self.AllowLeft`)
          (`self.K2_AddActorLocalOffset` (`self.Sidewalk`) true))))
    (:`then_3`
      ;[1 1 1] MoveRight
      (if (and (`self.AllowRight`) (`self.Sprinting`))
        (`self.K2_AddActorLocalOffset` (* (`self.Strafe`) -1) true)
        (elif (`self.AllowRight`)
          (`self.K2_AddActorLocalOffset` (* (`self.Sidewalk`) -1) true))))))

(event `self.ReceiveBeginPlay`
  ;[1 1 1] StartSettings
  (set `self.Speed` (`self.Walk`))
  ;[1 1 1] LightFlicker
  (bind (_direction _flicker) (`Timeline|Light Flicker`)
    (:`Update`
      (`LightComponent.SetIntensity` (`self.Light`) (* (`self.LightIntensity`) _flicker)))))

(event `InputAction|Forward`
  (params (Key :type "Key Structure"))
  ;[1 1 1] MoveForward
  (:`Pressed`
    (set `self.AllowForward` true))
  (:`Released`
    (set `self.AllowForward` false)))

(event `InputAction|Sprint`
  (params (Key :type "Key Structure"))
  ;[1 1 1] Sprint
  (:`Pressed`
    (set `self.Speed` (`self.Sprint`))
    (set `self.Sprinting` true))
  (:`Released`
    (set `self.Speed` (`self.Walk`))
    (set `self.Sprinting` false)))

(event `InputAction|Backward`
  (params (Key :type "Key Structure"))
  ;[1 1 1] MoveBackward
  (:`Pressed`
    (set `self.AllowBackward` true))
  (:`Released`
    (set `self.AllowBackward` false)))

(event `InputAction|Left`
  (params (Key :type "Key Structure"))
  ;[1 1 1] MoveLeft
  (:`Pressed`
    (set `self.AllowLeft` true))
  (:`Released`
    (set `self.AllowLeft` false)))

(event `InputAction|Right`
  (params (Key :type "Key Structure"))
  ;[1 1 1] MoveRight
  (:`Pressed`
    (set `self.AllowRight` true))
  (:`Released`
    (set `self.AllowRight` false)))

(fn `UserConstructionScript`)